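; Package spawner actor that presents the game's packages one at a time, alongside a cage component.
; New Game runs Setup with level data, and each pickup reported by PackagePool removes the first queued package and spawns the next.
; SpawnPackage resets the package's rotation and positions it relative to the spawner using an offset scaled by its integer size.
; Pause and Finish return all packages and hide the cage, while UnPause shows it and spawns again.
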(event `self.NewGame`
  ;[1 1 1] New Game
  (`self.Setup` (`BilpakkGameState.GetLevelData`))
  (`SceneComponent.SetVisibility` (`self.Cage`) true true)
  (`self.SpawnPackage`))

(event `self.Pause`
  ;[1 1 1] Pause
  (`PackagePool.ReturnAllPackages` (`self.PackagePool`))
  (`SceneComponent.SetVisibility` (`self.Cage`) false true))

(event `self.PackagePool.OnPackageInteracted`
  ;[1 1 1] Get next package when previous is picked up
  (`self.RemoveFirstPackageFromQueue`)
  (`self.SpawnPackage`))

(event `self.UnPause`
  ;[1 1 1] UnPause
  (`SceneComponent.SetVisibility` (`self.Cage`) true true)
  (`self.SpawnPackage`))

(event `self.Finish`
  ;[1 1 1] Finish Game
  (`PackagePool.ReturnAllPackages` (`self.PackagePool`))
  (`SceneComponent.SetVisibility` (`self.Cage`) false true))

(fn `UserConstructionScript`)