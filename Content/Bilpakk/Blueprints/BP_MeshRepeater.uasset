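; BP_MeshRepeater is an actor that repeats one mesh across a flat grid.
; Its construction script assigns the Mesh and Material variables to an InstancedStaticMesh component.
; Nested loops over GridX and GridY then add instances in local X and Y, spaced by Size, with the component handling instanced rendering.
; The event graph holds only disabled placeholder events, so the actor has no gameplay logic.
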(fn `UserConstructionScript`
  (bind _instancedstaticmesh (`self.InstancedStaticMesh`))
  (bind _size (`self.Size`))
  (`StaticMeshComponent.SetStaticMesh` _instancedstaticmesh (`self.Mesh`))
  (`PrimitiveComponent.SetMaterial` _instancedstaticmesh 0 (`self.Material`))
  (for _index (range (+ (`self.GridX`) 1))
    (for _index_2 (range (+ (`self.GridY`) 1))
      (`InstancedStaticMeshComponent.AddInstance` _instancedstaticmesh (`KismetMathLibrary.MakeTransform` (`KismetMathLibrary.MakeVector` (`KismetMathLibrary.Conv_IntToDouble` (* _index _size)) (`KismetMathLibrary.Conv_IntToDouble` (* _index_2 _size))))))))