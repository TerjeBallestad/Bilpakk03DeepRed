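; BP_StackingHandController is a VR motion-controller hand for interacting with stackable packages.
; On BeginPlay it caches the glove anim Blueprint and, after a short delay, mirrors the hand mesh for the left hand via negative Z scale.
; Every tick it copies GripState into the anim Blueprint.
; When the interaction collider begins overlapping a StackablePackage, it plays a half-strength haptic pulse on that hand.
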(event `self.ReceiveBeginPlay`
  (bind _asabp_glove_grip (cast `/Game/Bilpakk/SkeletalMeshes/Animations/ABP_GloveGrip` (`SkeletalMeshComponent.GetAnimInstance` (`self.HandMesh`))))
  (set `self.GloveAnimBP` _asabp_glove_grip)
  (`KismetSystemLibrary.Delay` 0.2)
  ;[1 1 1] Flip left hand mesh
  (if (== (`MotionControllerComponent.MotionSource` (`self.MotionControllerComponent`)) "Left")
    (`SceneComponent.SetWorldScale3D` (`self.HandMesh`) (1.0 1.0 -1.0))))

(event `RumbleController`
  (params (Intensity :type "Float (double-precision)"))
  ;[1 1 1] Rumble Controller
  (`PlayerController.PlayHapticEffect` (`GameplayStatics.GetPlayerController` 0) "/Game/Bilpakk/Data/MotionControllerHaptics.MotionControllerHaptics" (`MotionControllerComponent.Hand` (`self.MotionControllerComponent`)) Intensity false))

(event `self.InteractionCollider.OnComponentBeginOverlap`
  (params (OverlappedComponent :type "PrimitiveComponent Object Reference") (OtherActor :type "Actor Object Reference") (OtherComp :type "PrimitiveComponent Object Reference") (OtherBodyIndex :type Integer) (bFromSweep :type Boolean) (SweepResult :type "HitResult Structure (by ref)"))
  (cast `StackablePackage` OtherActor)
  (`self.RumbleController` 0.5))

(event `self.ReceiveTick`
  (params (DeltaSeconds :type "Float (single-precision)"))
  (set `/Game/Bilpakk/SkeletalMeshes/Animations/ABP_GloveGrip.GripState` (`self.GripState`) (`self.GloveAnimBP`)))

(fn `UserConstructionScript`)