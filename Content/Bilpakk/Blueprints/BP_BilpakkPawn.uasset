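; BP_BilpakkPawn is the pawn for the Bilpakk game, with left and right hand controllers that can hold packages.
; Its NewGame event runs SetupMap.
; When OnSetHidden fires, it casts each controller to BP_StackingHandController, then detaches any valid active package and returns it to the package pool.
; The right hand is handled before the left, with a debug print for each returned package.
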(event `self.NewGame`
  (`self.SetupMap`))

(event `self.OnSetHidden`
  (`|ExecutionSequence`
    (:`then_0`
      (bind _asbp_stacking_hand_controller (cast `/Game/Bilpakk/Blueprints/BP_StackingHandController` (`self.RightHandController`)))
      (bind _activepackage (`HandController.ActivePackage` _asbp_stacking_hand_controller))
      (`/Engine/EditorBlueprintResources/StandardMacros.IsValid` _activepackage
        (:`Is Valid`
          (`self.K2_DetachFromActor` _activepackage "KeepWorld" "KeepWorld" "KeepWorld")
          (`StackablePackage.ReturnToPackagePool` _activepackage)
          (`KismetSystemLibrary.PrintString` "Return to package pool"))))
    (:`then_1`
      (bind _asbp_stacking_hand_controller_2 (cast `/Game/Bilpakk/Blueprints/BP_StackingHandController` (`self.LeftHandController`)))
      (bind _activepackage_2 (`HandController.ActivePackage` _asbp_stacking_hand_controller_2))
      (`/Engine/EditorBlueprintResources/StandardMacros.IsValid` _activepackage_2
        (:`Is Valid`
          (`self.K2_DetachFromActor` _activepackage_2 "KeepWorld" "KeepWorld" "KeepWorld")
          (`StackablePackage.ReturnToPackagePool` _activepackage_2)
          (`KismetSystemLibrary.PrintString` "Return to package pool"))))))

(fn `UserConstructionScript`)