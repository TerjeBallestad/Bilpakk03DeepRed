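; BP_UIHandController is a VR hand controller actor with a laser pointer for interacting with widget UI.
; Shortly after BeginPlay, it picks the left or right Touch controller mesh from the motion controller's MotionSource.
; Each tick, Pointer hit results position an endpoint marker and stretch the pointer mesh along X to the hit distance.
; Off hit-testable widgets, the marker hides and the beam extends to the full interaction distance.
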(event `self.ReceiveBeginPlay`
  (bind _controllermesh (`self.ControllerMesh`))
  (`KismetSystemLibrary.Delay` 0.2)
  ;[1 1 1] Set correct controller mesh to each hand
  (switch `name` (`MotionControllerComponent.MotionSource` (`self.MotionControllerComponent`))
    (:`Left`
      (`StaticMeshComponent.SetStaticMesh` _controllermesh "/Game/Bilpakk/StaticMeshes/LeftTouchForQuestRiftSController.LeftTouchForQuestRiftSController"))
    (:`Right`
      (`StaticMeshComponent.SetStaticMesh` _controllermesh "/Game/Bilpakk/StaticMeshes/RightTouchForQuestRiftSController.RightTouchForQuestRiftSController"))))

(event `self.ReceiveTick`
  (params (DeltaSeconds :type "Float (single-precision)"))
  (bind _pointer (`self.Pointer`))
  (bind _endpointmesh (`self.EndpointMesh`))
  (bind _pointermesh (`self.PointerMesh`))
  (bind (_returnvalue_bblockinghit _returnvalue_binitialoverlap _returnvalue_time _returnvalue_distance _returnvalue_location) (`GameplayStatics.BreakHitResult` (`WidgetInteractionComponent.GetLastHitResult` _pointer)))
  (if (`WidgetInteractionComponent.IsOverHitTestVisibleWidget` _pointer)
    (`SceneComponent.SetVisibility` _endpointmesh true true)
    (`SceneComponent.K2_SetWorldLocation` _endpointmesh _returnvalue_location false false)
    (`SceneComponent.SetWorldScale3D` _pointermesh (`KismetMathLibrary.MakeVector` _returnvalue_distance 1.0 1.0))
    (else
      (`SceneComponent.SetVisibility` _endpointmesh false false)
      (`SceneComponent.SetWorldScale3D` _pointermesh (`KismetMathLibrary.MakeVector` (`WidgetInteractionComponent.InteractionDistance` _pointer) 1.0 1.0)))))

(fn `UserConstructionScript`)