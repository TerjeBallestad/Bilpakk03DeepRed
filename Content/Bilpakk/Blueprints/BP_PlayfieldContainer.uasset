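; Playfield container for the Bilpakk package-stacking game, managing a round's car model, level setup, timer and score display.
; New game, pause, unpause and finish events toggle visibility and the Tick-driven clock, with finish and non-first new games clearing stacked packages.
; A delayed 3-2-1 countdown starts the clock.
; Score changes update the points plate and animate separately styled positive and negative floating-text widgets through a timeline.
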(event `self.NewGame`
  (bind _returnvalue (`BilpakkGameState.GetLevelData`))
  (bind _3_2_1floatingtextwidget (`self.3-2-1FloatingTextWidget`))
  (bind _pointsplatewidget (`self.PointsPlateWidget`))
  ;[1 1 1] New Game
  (if (`self.FirstTime`)
    (set `self.FirstTime` false)
    (else
      (`self.Setup` _returnvalue)
      (`ActorPool.ClearStackedPackages` (`self.StaticMeshPool`))
      (`SceneComponent.SetVisibility` (`self.CarModel`) true true)
      (`TextBlock.SetText` (`/Game/Bilpakk/UI/Widgets/WBP_PointsPlate.LevelLabel` _pointsplatewidget) (`.LevelName` (break `BilpakkLevel` _returnvalue)))
      (`TextBlock.SetText` (`/Game/Bilpakk/UI/Widgets/WBP_PointsPlate.PointsLabel_1` _pointsplatewidget) (`KismetTextLibrary.Conv_IntToText` (`BilpakkGameState.GetPoints`)))
      (set `self.PreviousPoints` 0)
      (set `self.TimeSec` 0.0)
      (set `self.TimeMin` 0)
      (`self.UpdateTimeLabels`)
      (`KismetSystemLibrary.Delay` 2.0)
      (`self.3-2-1-go`)
      (bind (_direction _up _opacity) (`Timeline|Timeline_0` :!via `PlayFromStart`)
        (:`Update`
          (`Widget.SetRenderOpacity` _3_2_1floatingtextwidget _opacity))
        (:`Finished`
          (`self.SetFontSize` (`/Game/Bilpakk/UI/Widgets/WBP_FloatingText.Label` _3_2_1floatingtextwidget) 24))))))

(event `self.Pause`
  ;[1 1 1] Pause
  (`SceneComponent.SetVisibility` (`self.CarModel`) false true)
  (`SceneComponent.SetVisibility` (`self.PreviewMesh`) false true)
  (set `self.ShouldCountTime` false))

(event `self.ReceiveBeginPlay`
  ;[0.5669 1 0.6273] Setup
  (add `self.OnPointsAdded` (delegate `UpdatePoints`))
  (`|ExecutionSequence`
    (:`then_0`
      (bind _aswbp_points_plate (cast `/Game/Bilpakk/UI/Widgets/WBP_PointsPlate` (`WidgetComponent.GetUserWidgetObject` (`self.PointsWidget`))))
      (set `self.PointsPlateWidget` _aswbp_points_plate))
    (:`then_1`
      (bind _aswbp_floating_text (cast `/Game/Bilpakk/UI/Widgets/WBP_FloatingText` (`WidgetComponent.GetUserWidgetObject` (`self.FloatingTextWidget`))))
      (bind _output_get (set `self.FloatingTextWBP` _aswbp_floating_text))
      (`self.SetFontColorAndOutline` (`/Game/Bilpakk/UI/Widgets/WBP_FloatingText.Label` _output_get) (`self.PositiveOutline`) (`self.PositiveColors`))
      (`Widget.SetRenderOpacity` _output_get 0.0))
    (:`then_2`
      (bind _aswbp_floating_text_2 (cast `/Game/Bilpakk/UI/Widgets/WBP_FloatingText` (`WidgetComponent.GetUserWidgetObject` (`self.3-2-1FloatingText`))))
      (set `self.3-2-1FloatingTextWidget` _aswbp_floating_text_2))
    (:`then_3`
      (bind _aswbp_floating_text_3 (cast `/Game/Bilpakk/UI/Widgets/WBP_FloatingText` (`WidgetComponent.GetUserWidgetObject` (`self.NegativeFloatingTextWidget`))))
      (bind _output_get_2 (set `self.NegativeFloatingWidget` _aswbp_floating_text_3))
      (`self.SetFontColorAndOutline` (`/Game/Bilpakk/UI/Widgets/WBP_FloatingText.Label` _output_get_2) (`self.NegativeOutline`) (`self.NegativeColors`))
      (`Widget.SetRenderOpacity` _output_get_2 0.0))))

(event `self.UnPause`
  ;[1 1 1] UnPause
  (`SceneComponent.SetVisibility` (`self.CarModel`) true true)
  (set `self.ShouldCountTime` true))

(event `UpdatePoints`
  (bind (_points_total _points_negative _points_bonus _points_diff) (break `Points` (`self.Points`)))
  (bind _floatingtextwidget (`self.FloatingTextWidget`))
  (bind _negativefloatingtextwidget (`self.NegativeFloatingTextWidget`))
  ;[1 1 1] Update Points
  (`TextBlock.SetText` (`/Game/Bilpakk/UI/Widgets/WBP_PointsPlate.PointsLabel_1` (`self.PointsPlateWidget`)) (`KismetTextLibrary.Conv_IntToText` (`BilpakkGameState.GetPoints`)))
  (`TextBlock.SetText` (`/Game/Bilpakk/UI/Widgets/WBP_FloatingText.Label` (`self.FloatingTextWBP`)) (`KismetTextLibrary.Conv_IntToText` _points_diff))
  (`TextBlock.SetText` (`/Game/Bilpakk/UI/Widgets/WBP_FloatingText.Label` (`self.NegativeFloatingWidget`)) (`KismetTextLibrary.Conv_IntToText` _points_negative))
  (bind (_direction _up _opacity _down) (`Timeline|FloatingText` :!via `PlayFromStart`)
    (:`Update`
      (`SceneComponent.K2_AddRelativeLocation` _floatingtextwidget (`KismetMathLibrary.MakeVector` 0.0 0.0 _up) false false)
      (if (> _points_diff 0)
        (`Widget.SetRenderOpacity` (`WidgetComponent.GetWidget` _floatingtextwidget) _opacity))
      (if (or (< _points_negative 0) (and (== _points_negative 0) (== _points_diff 0)))
        (`Widget.SetRenderOpacity` (`WidgetComponent.GetWidget` _negativefloatingtextwidget) _opacity)
        (`SceneComponent.K2_AddRelativeLocation` _negativefloatingtextwidget (`KismetMathLibrary.MakeVector` 0.0 0.0 _down) false false)))
    (:`Finished`)))

(event `self.Finish`
  ;[1 1 1] Finish game
  (`ActorPool.ClearStackedPackages` (`self.StaticMeshPool`))
  (`SceneComponent.SetVisibility` (`self.CarModel`) false true)
  (set `self.ShouldCountTime` false))

(event `self.ReceiveTick`
  (params (DeltaSeconds :type "Float (single-precision)"))
  ;[1 1 1] Timer
  (if (`self.ShouldCountTime`)
    (bind _output_get (set `self.TimeSec` (/ (`KismetMathLibrary.Conv_IntToDouble` (`KismetMathLibrary.FFloor` (* (+ DeltaSeconds (`self.TimeSec`)) 100.0))) 100.0)))
    (if (> _output_get 59.0)
      (`/Engine/EditorBlueprintResources/StandardMacros.IncrementInt` (`self.TimeMin`)
        (:`  `
          (set `self.TimeSec` 0.0))))
    (`self.UpdateTimeLabels`)))

(fn `UpdateTimeLabels`
  (`TextBlock.SetText` (`/Game/Bilpakk/UI/Widgets/WBP_PointsPlate.TimeLabel` (`self.PointsPlateWidget`)) (`|FormatText` "{min}:{sec}" (`KismetStringLibrary.Right` (`KismetStringLibrary.Concat_StrStr` "0" (`KismetStringLibrary.Conv_IntToString` (`self.TimeMin`))) 2) (`self.TimeSec`))))

(fn `UserConstructionScript`)