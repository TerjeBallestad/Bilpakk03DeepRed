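; Preview container that lays out a level's SpawnQueue of packages inside a row of cages.
; On SetupLevelData it resets the actor pool, then draws pooled meshes for cages and scaled packages, each cage getting its own package grid.
; Packing is greedy: each unrotated package tests every X/Y cell and takes the lowest-Z fit, marking those cells.
; When nothing fits, it spawns another cage alongside and retries there.
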(event `SetupLevelData`
  (params (LevelData :type "BilpakkLevel Structure"))
  (bind _currentgrid (`self.CurrentGrid`))
  (bind (_lowestlocation_x _lowestlocation_y _lowestlocation_z) (`KismetMathLibrary.BreakVector` (`self.LowestLocation`)))
  (bind _inouttransform_location (`KismetMathLibrary.BreakTransform` (`self.InOutTransform`)))
  (bind _currentgrid_2 (`self.CurrentGrid`))
  (bind _packagescale (`self.PackageScale`))
  (bind (_size_x _size_y) (break `IntVector` (`PackageGrid.Size` _currentgrid)))
  (set `self.NumCages` 0)
  (`ActorPool.ClearStackedPackages` (`self.ActorPool`))
  (`self.Setup` LevelData)
  (`self.SpawnCage`)
  (for _array_element (`self.SpawnQueue`)
    (set `self.LowestLocation` (99999.0 9999999.0 99999.0) :!label _label)
    (set `self.FoundSpace` false)
    (`|ExecutionSequence`
      (:`then_0`
        (bind _returnvalue (`ActorPool.GetPooledActor` (`self.ActorPool`)))
        (`SceneComponent.SetVisibility` _returnvalue false true)
        (bind (_sizee _sizeint _type _mesh _material) (break `PackageParameters` _array_element))
        (`StaticMeshComponent.SetStaticMesh` _returnvalue _mesh)
        (`PrimitiveComponent.SetMaterial` _returnvalue 0 _material)
        (`SceneComponent.SetWorldScale3D` _returnvalue (* (1.0 1.0 1.0) _packagescale))
        (for _index (range (+ _size_x 1))
          (for _index_2 (range (+ _size_y 1))
            (bind _returnvalue_2 (`KismetMathLibrary.MakeTransform` (`PackageGrid.GridToWorldLocation` _currentgrid (make `IntVector` _index _index_2))))
            (bind (_min _max) (`StaticMeshComponent.GetLocalBounds` _returnvalue))
            (bind _outrange (`PackageGrid.CalculatePackageBounds` _currentgrid_2 _returnvalue_2 (* _min _packagescale) (* _max _packagescale)))
            (bind _output_get (set `self.InOutRange` _outrange))
            (bind _returnvalue_3 (`PackageGrid.FindSpaceForPackage` _currentgrid_2 _returnvalue_2 _output_get (`self.InOutTransform`)))
            (if _returnvalue_3
              (if (< (.z (.location (`self.InOutTransform`))) _lowestlocation_z)
                (set `self.LowestLocation` _inouttransform_location)
                (set `self.LowestRange` (`self.InOutRange`))
                (set `self.FoundSpace` true))))))
      (:`then_1`
        (if (`self.FoundSpace`)
          (`SceneComponent.K2_SetWorldLocation` _returnvalue (`self.LowestLocation`) false false)
          (`SceneComponent.SetVisibility` _returnvalue true true)
          (`PackageGrid.SetStatus` (`self.CurrentGrid`) (`self.LowestRange`) _type)
          (else
            (`self.SpawnCage`)
            (goto _label)))))))

(event `self.ReceiveTick`
  (params (DeltaSeconds :type "Float (single-precision)")))

(fn `UserConstructionScript`)